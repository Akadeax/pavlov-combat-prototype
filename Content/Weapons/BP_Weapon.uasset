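; BP_Weapon is a data-driven hitscan weapon that takes its mesh and firing stats from WeaponData.
; TryFire checks fire delay and optional limited ammo, then ShootBullet line-traces from the camera with random inaccuracy and spawns muzzle and beam-trail effects.
; Hit BPI_Shootable actors receive OnShot, with "Head" bone hits counting as crits.
; Tick tracks time since the last shot and gradually recharges limited ammo after firing pauses.
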(event `self.ReceiveBeginPlay`
  (`SkeletalMeshComponent.SetSkeletalMeshAsset` (`self.WeaponMesh`) (`/Game/Weapons/BP_WeaponData.Mesh` (`self.WeaponData`)))
  (if (`/Game/Weapons/BP_WeaponData.LimitedAmmo` (`self.WeaponData`))
    _))

(event `self.ReceiveTick`
  (params (DeltaSeconds :type "Float (single-precision)"))
  (bind _weapondata (`self.WeaponData`))
  (`|ExecutionSequence`
    (:`then_0`
      (set `self.TimeSinceLastShot` (+ (`self.TimeSinceLastShot`) DeltaSeconds)))
    (:`then_1`
      (if (and (`/Game/Weapons/BP_WeaponData.LimitedAmmo` _weapondata) (< (`self.CurrentAmmoLeft`) (`/Game/Weapons/BP_WeaponData.MaxAmmo` _weapondata)) (> (`self.TimeSinceLastShot`) (* (`/Game/Weapons/BP_WeaponData.FireDelay` (`self.WeaponData`)) 1.2)))
        (bind _output_get (set `self.TimeSinceLastAmmoGained` (+ (`self.TimeSinceLastAmmoGained`) DeltaSeconds)))
        (if (>= _output_get (`/Game/Weapons/BP_WeaponData.AmmoRechargeInterval` (`self.WeaponData`)))
          (set `self.TimeSinceLastAmmoGained` 0.0)
          (`/Engine/EditorBlueprintResources/StandardMacros.IncrementInt` (`self.CurrentAmmoLeft`)))))))

(fn `ShootBullet`
  (bind _camera (`self.Camera`))
  (bind _weapondata (`self.WeaponData`))
  (bind _returnvalue (`SceneComponent.K2_GetComponentLocation` _camera))
  (`NiagaraFunctionLibrary.SpawnSystemAttached` "/Game/Weapons/FXS_WeaponShoot.FXS_WeaponShoot" (`self.WeaponMesh`) "Muzzle" (0.0 0.0 0.0) (struct) "SnapToTargetIncludingScale" true true "AutoRelease")
  (bind (_outhit _returnvalue_2) (`KismetSystemLibrary.LineTraceSingle` _returnvalue (+ _returnvalue (* (`/Game/BML_WeaponMath.AddInnacuracy` (`KismetMathLibrary.GetForwardVector` (`SceneComponent.K2_GetComponentRotation` _camera)) (`/Game/Weapons/BP_WeaponData.InnacuracyDegrees` (`self.WeaponData`))) 5000.0)) "TraceTypeQuery3" false (`|MakeArray` (`ActorComponent.GetOwner` (`self.Camera`)))))
  (`self.SpawnBulletTrail` _outhit)
  (if _returnvalue_2
    (bind (_bblockinghit _binitialoverlap _time _distance _location _impactpoint _normal _impactnormal _physmat _hitactor _hitcomponent _hitbonename) (`GameplayStatics.BreakHitResult` _outhit))
    (bind _asbpi_shootable (cast `/Game/Enemies/BPI_Shootable` _hitactor))
    (bind _returnvalue_3 (select `bool` (== _hitbonename "Head") :`false` "NewEnumerator1" :`true` "NewEnumerator2" :!type "/Game/Weapons/E_WeaponHitType Enum"))
    (`/Game/Enemies/BPI_Shootable.OnShot` _asbpi_shootable (`ActorComponent.GetOwner` (`self.Camera`)) _returnvalue_3 (select `/Game/Weapons/E_WeaponHitType` _returnvalue_3 :`NewEnumerator1` (`/Game/Weapons/BP_WeaponData.Damage` _weapondata) :`NewEnumerator2` (`/Game/Weapons/BP_WeaponData.CritDamage` _weapondata)))))

(fn `SpawnBulletTrail`
  (params (HitResult :type "HitResult Structure"))
  (locals (TargetWorldPos :type "Vector Structure"))
  (bind (_bblockinghit _binitialoverlap _time _distance _location _impactpoint _normal _impactnormal _physmat _hitactor _hitcomponent _hitbonename _bonename _hititem _elementindex _faceindex _tracestart _traceend) (`GameplayStatics.BreakHitResult` HitResult))
  (if _bblockinghit
    (set `local.TargetWorldPos` _impactpoint)
    (else
      (set `local.TargetWorldPos` _traceend)))
  (bind _returnvalue (`NiagaraFunctionLibrary.SpawnSystemAtLocation` "/Game/Character/FXS_WeaponBulletTrail.FXS_WeaponBulletTrail" (`SceneComponent.GetSocketLocation` (`self.WeaponMesh`) "Muzzle") (struct) (1.0 1.0 1.0) true true "AutoRelease"))
  (`NiagaraComponent.SetVariableVec3` _returnvalue "BeamEnd" (`local.TargetWorldPos`)))

(fn `TryFire`
  (returns (Success :type Boolean) (WeaponData :type "/Game/Weapons/BP_WeaponData Object Reference"))
  (if (and (not (`self.InFireDelay`)) (or (not (`/Game/Weapons/BP_WeaponData.LimitedAmmo` (`self.WeaponData`))) (> (`self.CurrentAmmoLeft`) 0)))
    (if (`/Game/Weapons/BP_WeaponData.LimitedAmmo` (`self.WeaponData`))
      (`/Engine/EditorBlueprintResources/StandardMacros.DecrementInt` (`self.CurrentAmmoLeft`)
        (:`  `
          _)))
    (set `self.TimeSinceLastShot` 0.0)
    (`self.ShootBullet`)
    (return true (`self.WeaponData`))
    (else
      (return false null))))

(fn `UserConstructionScript`)
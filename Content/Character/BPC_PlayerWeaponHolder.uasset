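; Player weapon holder component that spawns a pistol and rifle on BeginPlay and handles switching and firing input.
; Each weapon is a BP_Weapon built from a data asset, given the tagged player camera, attached hidden to the arm mesh's Hand socket.
; Equipping swaps visibility by slot index.
; Press input fires non-automatic weapons and hold input fires automatic ones, both through TryFire on the equipped weapon.
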(event `self.ReceiveBeginPlay`
  (`self.Set Weapon` "/Game/Weapons/Pistol/DA_WeaponPistol.DA_WeaponPistol")
  (`self.Set Weapon` "/Game/Weapons/Rifle/DA_WeaponRifle.DA_WeaponRifle" 1))

(event `EnhancedInput|/Game/Input/Actions/IA_FirstWeapon`
  (params (ActionValue :type Boolean) (ElapsedSeconds :type "Float (double-precision)") (TriggeredSeconds :type "Float (double-precision)") (InputAction :type "InputAction Object Reference" :default "/Game/Input/Actions/IA_FirstWeapon.IA_FirstWeapon"))
  (:`Triggered`
    (`self.EquipWeapon` 0)))

(event `EnhancedInput|/Game/Input/Actions/IA_SecondWeapon`
  (params (ActionValue :type Boolean) (ElapsedSeconds :type "Float (double-precision)") (TriggeredSeconds :type "Float (double-precision)") (InputAction :type "InputAction Object Reference" :default "/Game/Input/Actions/IA_SecondWeapon.IA_SecondWeapon"))
  (:`Triggered`
    (`self.EquipWeapon` 1)))

(event `EnhancedInput|/Game/Input/Actions/IA_ShootPress`
  (params (ActionValue :type Boolean) (ElapsedSeconds :type "Float (double-precision)") (TriggeredSeconds :type "Float (double-precision)") (InputAction :type "InputAction Object Reference" :default "/Game/Input/Actions/IA_ShootPress.IA_ShootPress"))
  (bind _weapon (`self.GetEquippedWeapon`))
  ;[0.2292 0.2292 0.2292] ShootInput
  (:`Triggered`
    ;;[0 0 0] Support hold for automatic weapons & down for non-automatic
    (`/Engine/EditorBlueprintResources/StandardMacros.IsValid` _weapon
      (:`Is Valid`
        (if (not (`/Game/Weapons/BP_WeaponData.Automatic` (`/Game/Weapons/BP_Weapon.WeaponData` _weapon)))
          (`/Game/Weapons/BP_Weapon.TryFire` (`self.GetEquippedWeapon`) :!label _label))))))

(event `EnhancedInput|/Game/Input/Actions/IA_ShootHold`
  (params (ActionValue :type Boolean) (ElapsedSeconds :type "Float (double-precision)") (TriggeredSeconds :type "Float (double-precision)") (InputAction :type "InputAction Object Reference" :default "/Game/Input/Actions/IA_ShootHold.IA_ShootHold"))
  (bind _weapon (`self.GetEquippedWeapon`))
  ;[0.2292 0.2292 0.2292] ShootInput
  (:`Triggered`
    ;;[0 0 0] Support hold for automatic weapons & down for non-automatic
    (`/Engine/EditorBlueprintResources/StandardMacros.IsValid` _weapon
      (:`Is Valid`
        (if (`/Game/Weapons/BP_WeaponData.Automatic` (`/Game/Weapons/BP_Weapon.WeaponData` _weapon))
          (goto _label))))))

(fn `EquipWeapon`
  (params (Index :type Integer))
  (locals (NewLocalVar :type Integer))
  (if (!= Index (`self.EquippedWeaponIndex`))
    (if (!= (`self.EquippedWeaponIndex`) -1)
      (`self.SetWeaponHidden` (`self.EquippedWeaponIndex`) true))
    (bind _output_get (set `self.EquippedWeaponIndex` Index))
    (`self.SetWeaponHidden` _output_get)))

(fn `Set Weapon`
  (params (Data :type "/Game/Weapons/BP_WeaponData Object Reference") (Index :type Integer))
  (bind _returnvalue (`|SpawnActorFromClass` "/Game/Weapons/BP_Weapon.BP_Weapon_C" (`Actor.GetTransform` (`self.GetOwner`)) "AlwaysSpawn" "MultiplyWithRoot" null Data (`Actor.FindComponentByTag` (`self.GetOwner`) "/Script/Engine.CameraComponent" "PlayerCam") null))
  (`Actor.K2_AttachToComponent` _returnvalue (`Actor.FindComponentByTag` (`self.GetOwner`) "/Script/Engine.SkeletalMeshComponent" "ArmMesh") "Hand" "SnapToTarget" "SnapToTarget" "KeepRelative" false)
  (`KismetArrayLibrary.Array_Set` (`self.EquippedWeapons`) Index _returnvalue true)
  (`Actor.SetActorHiddenInGame` _returnvalue true))

(fn `SetWeaponHidden`
  (params (Index :type Integer) (NewHidden :type Boolean))
  (`Actor.SetActorHiddenInGame` (`|GetArrayItem` (`self.EquippedWeapons`) Index) NewHidden))
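; BP_Revolver is a hitscan revolver weapon that fires from the player's camera, with a cooldown between shots.
; TryShoot fires only when the Tick-decremented cooldown has expired, then resets it and returns whether it fired.
; DoShot line-traces forward from the camera, ignoring the player and drawing debug lines.
; Hit actors receive OnShotMessage with the shooter and a crit flag for "Head" bone hits.
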(event `self.ReceiveTick`
  (params (DeltaSeconds :type "Float (single-precision)"))
  (bind _currentshotcooldown (`self.CurrentShotCooldown`))
  (if (> _currentshotcooldown 0.0)
    (set `self.CurrentShotCooldown` (- _currentshotcooldown DeltaSeconds))))

(fn `DoShot`
  (bind _asbp_player_character (cast `/Game/Character/BP_PlayerCharacter` (`GameplayStatics.GetPlayerPawn` 0)))
  (bind _camera (`/Game/Character/BP_PlayerCharacter.Camera` _asbp_player_character))
  (bind _returnvalue (`SceneComponent.K2_GetComponentLocation` _camera))
  (bind (_outhit _returnvalue_2) (`KismetSystemLibrary.LineTraceSingle` _returnvalue (+ _returnvalue (* (`KismetMathLibrary.GetForwardVector` (`SceneComponent.K2_GetComponentRotation` _camera)) 5000.0)) "TraceTypeQuery3" false (`|MakeArray` (`GameplayStatics.GetPlayerPawn` 0) :!type "Actor Object Reference") "ForDuration" true (struct :`R` 1.0 :`A` 1.0) (struct :`G` 1.0 :`A` 1.0) 2.0))
  (if _returnvalue_2
    (bind (_bblockinghit _binitialoverlap _time _distance _location _impactpoint _normal _impactnormal _physmat _hitactor _hitcomponent _hitbonename) (`GameplayStatics.BreakHitResult` _outhit))
    (message `/Game/Enemies/BPI_Shootable.OnShot` _hitactor (`GameplayStatics.GetPlayerPawn` 0) (== _hitbonename "Head"))))

(fn `TryShoot`
  (returns (Success :type Boolean))
  (if (<= (`self.CurrentShotCooldown`) 0.0)
    (`self.DoShot`)
    (set `self.CurrentShotCooldown` (`self.ShotCooldown`))
    (return true)
    (else
      (return false))))

(fn `UserConstructionScript`)
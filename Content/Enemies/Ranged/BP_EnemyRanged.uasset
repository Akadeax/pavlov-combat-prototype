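; BP_EnemyRanged is a ranged enemy character that reacts to being shot and is destroyed when health runs out.
; A surviving hit stuns it, launches it away from the shooter and plays a hurt montage, with stun and horizontal knockback scaled by impact.
; Stun writes a Blackboard duration that Tick counts down, and triggers a Timeline flash on a dynamic material created at BeginPlay.
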(event `/Game/Enemies/BPI_Shootable.OnShot`
  (params (ShotBy :type "Actor Object Reference") (HitType :type "/Game/Weapons/E_WeaponHitType Enum" :default "NewEnumerator0") (Damage :type Integer) (Impact :type "Float (double-precision)"))
  (bind _returnvalue (* (`self.HorizontalHitLaunch`) Impact))
  (bind (_returnvalue_x _returnvalue_y) (`KismetMathLibrary.BreakVector` (`KismetMathLibrary.Normal` (- (`self.K2_GetActorLocation`) (`self.K2_GetActorLocation` ShotBy)))))
  (bind _output_get (set `self.Health` (- (`self.Health`) Damage)))
  (if (<= _output_get 0)
    (`self.K2_DestroyActor`)
    (else
      (`self.Stun` (* Impact 0.1))
      (`self.LaunchCharacter` (`KismetMathLibrary.MakeVector` (* _returnvalue_x _returnvalue) (* _returnvalue_y _returnvalue) (`self.VerticalHitLaunch`)) true)
      (`|PlayMontage` (`self.Mesh`) "/Game/Enemies/Melee/Mesh/Animation/AM_EnemyHurt.AM_EnemyHurt"))))

(event `self.ReceiveTick`
  (params (DeltaSeconds :type "Float (single-precision)"))
  (`BlackboardComponent.SetValueAsFloat` (`AIBlueprintHelperLibrary.GetBlackboard` null) "StunDuration" (- (`BlackboardComponent.GetValueAsFloat` (`AIBlueprintHelperLibrary.GetBlackboard` null) "StunDuration") DeltaSeconds)))

(event `self.ReceiveBeginPlay`
  (bind _returnvalue (`KismetMaterialLibrary.CreateDynamicMaterialInstance` "/Game/Enemies/M_Enemy.M_Enemy"))
  (bind _output_get (set `self.Material` _returnvalue))
  (`PrimitiveComponent.SetMaterial` (`self.Mesh`) 0 _output_get))

(event `Flash`
  (bind (_direction _factor) (`Timeline|Timeline` :!via `PlayFromStart`)
    (:`Update`
      (`MaterialInstanceDynamic.SetScalarParameterValue` (`self.Material`) "FlashAlpha" _factor))))

(fn `Stun`
  (params (Duration :type "Float (double-precision)"))
  (`BlackboardComponent.SetValueAsFloat` (`AIBlueprintHelperLibrary.GetBlackboard` null) "StunDuration" Duration)
  (`self.Flash`))

(fn `UserConstructionScript`)
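; BP_EnemyMelee is a melee enemy character that hits the player on hurt box overlap, then knocks itself back and disables that box.
; Shots subtract health, doubled on crits, then either destroy it or stun it with knockback, a hurt montage and a disabled hurt box.
; Stun sets a Blackboard timer that Tick counts down, and flashes a dynamic material through a timeline.
; BeginPlay also halves global time dilation, affecting the whole game.
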(event `self.HurtBox.OnComponentBeginOverlap`
  (params (OverlappedComponent :type "PrimitiveComponent Object Reference") (OtherActor :type "Actor Object Reference") (OtherComp :type "PrimitiveComponent Object Reference") (OtherBodyIndex :type Integer) (bFromSweep :type Boolean) (SweepResult :type "HitResult Structure (by ref)"))
  (bind _horizontalhitlaunch (`self.HorizontalHitLaunch`))
  (bind _asbp_player_character (cast `/Game/Character/BP_PlayerCharacter` OtherActor))
  (`/Game/Character/BP_PlayerCharacter.OnHit` _asbp_player_character self)
  (`/Engine/EditorBlueprintResources/StandardMacros.IsValid` _asbp_player_character
    (:`Is Valid`
      (bind (_returnvalue_x _returnvalue_y) (`KismetMathLibrary.BreakVector` (`KismetMathLibrary.Normal` (- (`self.K2_GetActorLocation`) (`self.K2_GetActorLocation` _asbp_player_character)))))
      (`self.LaunchCharacter` (`KismetMathLibrary.MakeVector` (* _returnvalue_x _horizontalhitlaunch) (* _returnvalue_y _horizontalhitlaunch) (`self.VerticalHitLaunch`)) true true)
      (`self.SetHurtBoxEnabled` false))))

(event `/Game/Enemies/BPI_Shootable.OnShot`
  (params (ShotBy :type "Actor Object Reference") (Crit :type Boolean))
  (bind _horizontalhitlaunch (`self.HorizontalHitLaunch`))
  (bind (_returnvalue_x _returnvalue_y) (`KismetMathLibrary.BreakVector` (`KismetMathLibrary.Normal` (- (`self.K2_GetActorLocation`) (`self.K2_GetActorLocation` ShotBy)))))
  (bind _output_get (set `self.Health` (- (`self.Health`) (`KismetMathLibrary.SelectInt` 2 1 Crit))))
  (if (<= _output_get 0)
    (`self.K2_DestroyActor`)
    (else
      (`self.Stun` 1.0)
      (`self.SetHurtBoxEnabled` false)
      (`self.LaunchCharacter` (`KismetMathLibrary.MakeVector` (* _returnvalue_x _horizontalhitlaunch) (* _returnvalue_y _horizontalhitlaunch) (`self.VerticalHitLaunch`)) true)
      (`|PlayMontage` (`self.Mesh`) "/Game/Enemies/Melee/Mesh/Animation/AM_EnemyHurt.AM_EnemyHurt"))))

(event `self.ReceiveTick`
  (params (DeltaSeconds :type "Float (single-precision)"))
  (`BlackboardComponent.SetValueAsFloat` (`AIBlueprintHelperLibrary.GetBlackboard` null) "StunDuration" (- (`BlackboardComponent.GetValueAsFloat` (`AIBlueprintHelperLibrary.GetBlackboard` null) "StunDuration") DeltaSeconds)))

(event `self.ReceiveBeginPlay`
  (`GameplayStatics.SetGlobalTimeDilation` 0.5)
  (bind _returnvalue (`KismetMaterialLibrary.CreateDynamicMaterialInstance` "/Game/Enemies/M_Enemy.M_Enemy"))
  (bind _output_get (set `self.Material` _returnvalue))
  (`PrimitiveComponent.SetMaterial` (`self.Mesh`) 0 _output_get))

(event `Flash`
  (bind (_direction _factor) (`Timeline|FlashTimeline` :!via `PlayFromStart`)
    (:`Update`
      (`MaterialInstanceDynamic.SetScalarParameterValue` (`self.Material`) "FlashAlpha" _factor))))

(fn `SetHurtBoxEnabled`
  (params (Active :type Boolean))
  (`PrimitiveComponent.SetCollisionEnabled` (`self.HurtBox`) (select `bool` Active :`false` "NoCollision" :`true` "QueryOnly" :!type "ECollisionEnabled Enum")))

(fn `Stun`
  (params (Duration :type "Float (double-precision)"))
  (`BlackboardComponent.SetValueAsFloat` (`AIBlueprintHelperLibrary.GetBlackboard` null) "StunDuration" Duration)
  (`self.Flash`))

(fn `UserConstructionScript`)